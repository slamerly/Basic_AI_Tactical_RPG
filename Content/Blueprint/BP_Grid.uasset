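; Tile grid actor that builds a walkable map from the level and handles mouse-driven pathfinding between tiles.
; Construction script sphere-traces ground and obstacle channels into the TilesData map and draws debug planes; BeginPlay spawns a BP_Tile per entry.
; Hovering runs an A*-style, four-neighbour search with Manhattan heuristic from the selected tile and highlights the path.
; Selecting a tile passes the current path to BP_PlayerController.
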(event `self.ReceiveBeginPlay`
  (bind _returnvalue (`GameplayStatics.GetPlayerController` 0))
  ;[1 1 1] Mouse
  (set `PlayerController.bShowMouseCursor` true _returnvalue)
  (set `PlayerController.bEnableMouseOverEvents` true _returnvalue)
  (set `PlayerController.bEnableClickEvents` true _returnvalue)
  (`KismetSystemLibrary.FlushPersistentDebugLines`)
  ;[1 1 1] Spawn Tiles
  (bind _keys (`BlueprintMapLibrary.Map_Keys` (`self.TilesData`)))
  (for _array_element _keys
    (bind _value (`BlueprintMapLibrary.Map_Find` (`self.TilesData`) _array_element))
    (bind _returnvalue_2 (`|SpawnActorFromClass` "/Game/Blueprint/BP_Tile.BP_Tile_C" (`KismetMathLibrary.Conv_VectorToTransform` (`.WorldLocation_5_A610825A49763CE01582F8BE4E12333F` (break `/Game/Blueprint/Struct_Tile` _value))) "Undefined" "OverrideRootScale" null null))
    (set `/Game/Blueprint/BP_Tile.GridCoordinates` (`.Coordinates_8_53032BC04019C34375C23FA909D32976` (break `/Game/Blueprint/Struct_Tile` _value)) _returnvalue_2)
    (set `/Game/Blueprint/BP_Tile.Grid` self _returnvalue_2)
    (`BlueprintMapLibrary.Map_Add` (`self.TilesData`) (`.Coordinates_8_53032BC04019C34375C23FA909D32976` (break `/Game/Blueprint/Struct_Tile` _value)) (make `/Game/Blueprint/Struct_Tile` (break `/Game/Blueprint/Struct_Tile` _value) (`.WorldLocation_5_A610825A49763CE01582F8BE4E12333F` (break `/Game/Blueprint/Struct_Tile` _value)) (`.Coordinates_8_53032BC04019C34375C23FA909D32976` (break `/Game/Blueprint/Struct_Tile` _value)) _returnvalue_2))))

(event `OnNewTileSelected`
  (params (SelectedTile :type "/Game/Blueprint/BP_Tile Object Reference"))
  (bind _selectedtile (`self.SelectedTile`))
  (`/Engine/EditorBlueprintResources/StandardMacros.IsValid` _selectedtile
    (:`Is Valid`
      (if (not (== _selectedtile SelectedTile))
        (`/Game/Blueprint/BP_Tile.OnUnselectTile` _selectedtile)))
    (:`Is Not Valid`
      _))
  (set `self.SelectedTile` SelectedTile)
  (bind _asbp_player_controller (cast `/Game/Blueprint/BP_PlayerController` (`GameplayStatics.GetPlayerController` 0)))
  (`/Game/Blueprint/BP_PlayerController.OnNewPathAvailable` _asbp_player_controller (`self.Path`)))

(event `OnCurrentlyHoveredTile`
  (params (HoveredTile :type "/Game/Blueprint/BP_Tile Object Reference"))
  (bind _selectedtile (`self.SelectedTile`))
  (bind _hoveredtile (`self.HoveredTile`))
  (bind _returnvalue (and (`KismetSystemLibrary.IsValid` _selectedtile) (`KismetSystemLibrary.IsValid` _hoveredtile)))
  (`/Engine/EditorBlueprintResources/StandardMacros.IsValid` (`self.HoveredTile`)
    (:`Is Valid`
      _)
    (:`Is Not Valid`
      _))
  (set `self.HoveredTile` HoveredTile)
  (`self.HighlightCurrentPath` false)
  (if _returnvalue
    (`self.FindPath` (`/Game/Blueprint/BP_Tile.GridCoordinates` _selectedtile) (`/Game/Blueprint/BP_Tile.GridCoordinates` _hoveredtile))
    (`self.HighlightCurrentPath` _returnvalue)))

(fn `DrawTiles`
  (locals (X :type Integer) (Y :type Integer))
  (bind _values (`BlueprintMapLibrary.Map_Values` (`self.TilesData`)))
  (for _array_element _values
    (switch `/Game/Blueprint/Enum_GroundType` (break `/Game/Blueprint/Struct_Tile` _array_element)
      (:`NewEnumerator0`
        (`KismetSystemLibrary.DrawDebugPlane` (make `Plane` (.z (`.WorldLocation_5_A610825A49763CE01582F8BE4E12333F` (break `/Game/Blueprint/Struct_Tile` _array_element))) 0.0 0.0 1.0) (`.WorldLocation_5_A610825A49763CE01582F8BE4E12333F` (break `/Game/Blueprint/Struct_Tile` _array_element)) (- (`self.TileSize`) 5.0) (struct :`R` 1.0 :`G` 1.0 :`B` 1.0 :`A` 1.0) 100000.0))
      (:`NewEnumerator1`
        (`KismetSystemLibrary.DrawDebugPlane` (make `Plane` (.z (`.WorldLocation_5_A610825A49763CE01582F8BE4E12333F` (break `/Game/Blueprint/Struct_Tile` _array_element))) 0.0 0.0 1.0) (`.WorldLocation_5_A610825A49763CE01582F8BE4E12333F` (break `/Game/Blueprint/Struct_Tile` _array_element)) (- (`self.TileSize`) 5.0) (struct :`R` 0.109462 :`G` 0.039546 :`A` 1.0) 100000.0))
      (:`NewEnumerator2`
        (`KismetSystemLibrary.DrawDebugPlane` (make `Plane` (.z (`.WorldLocation_5_A610825A49763CE01582F8BE4E12333F` (break `/Game/Blueprint/Struct_Tile` _array_element))) 0.0 0.0 1.0) (`.WorldLocation_5_A610825A49763CE01582F8BE4E12333F` (break `/Game/Blueprint/Struct_Tile` _array_element)) (- (`self.TileSize`) 5.0) (struct :`A` 1.0) 100000.0)))))

(fn `FindPath`
  (params (StartCoords :type "Vector2D Structure") (GoalCoords :type "Vector2D Structure"))
  (locals (Start :type "Vector2D Structure") (Goal :type "Vector2D Structure") (OpenSet :type "Array of Vector2D Structure") (ClosedSet :type "Array of Vector2D Structure") (CurrentTile :type "Vector2D Structure") (CurrentNeighbour :type "Vector2D Structure") (OpenSetCheapest :type "Vector2D Structure") (CurrentNeighbourCostFromStart :type Integer))
  (bind _tilesdata (`self.TilesData`))
  (bind _tilesdata_2 (`self.TilesData`))
  (bind _tilesdata_3 (`self.TilesData`))
  (bind _tilesdata_4 (`self.TilesData`))
  (bind _start (`local.Start`))
  (bind _openset (`local.OpenSet`))
  (bind _value (`BlueprintMapLibrary.Map_Find` _tilesdata (`local.OpenSetCheapest`)))
  (bind _estimatedcost (`self.GetEstimatedCostToGoal` (`local.CurrentNeighbour`) (`local.Goal`)))
  (bind _value_2 (`BlueprintMapLibrary.Map_Find` _tilesdata_2 _start))
  (bind _estimatedcost_2 (`self.GetEstimatedCostToGoal` _start (`local.Goal`)))
  (bind _value_3 (`BlueprintMapLibrary.Map_Find` (`self.TilesData`) (`local.CurrentNeighbour`)))
  (set `local.Start` StartCoords)
  (set `local.Goal` GoalCoords)
  (if (`.ReturnValue` (`BlueprintMapLibrary.Map_Find` (`self.TilesData`) (`local.Goal`)))
    (`|ExecutionSequence`
      (:`then_0`
        ;[1 1 1] Default values - By adding, we replace the formerly modified values
        (bind _keys (`BlueprintMapLibrary.Map_Keys` (`self.TilesData`)))
        (for _array_element _keys
          (bind _value_4 (`BlueprintMapLibrary.Map_Find` _tilesdata_4 _array_element))
          (`BlueprintMapLibrary.Map_Add` _tilesdata_4 _array_element (make `/Game/Blueprint/Struct_Tile` (break `/Game/Blueprint/Struct_Tile` _value_4) (`.WorldLocation_5_A610825A49763CE01582F8BE4E12333F` (break `/Game/Blueprint/Struct_Tile` _value_4)) (`.Coordinates_8_53032BC04019C34375C23FA909D32976` (break `/Game/Blueprint/Struct_Tile` _value_4)) (`.TileActor_27_C837385A4995B3A36BD7829C414865E1` (break `/Game/Blueprint/Struct_Tile` _value_4)) (`.Cost_25_2C52E69A47A40DBB903D63AE9718D093` (break `/Game/Blueprint/Struct_Tile` _value_4)) 999 999 999)))
        (`BlueprintMapLibrary.Map_Add` _tilesdata_2 _start (make `/Game/Blueprint/Struct_Tile` (break `/Game/Blueprint/Struct_Tile` _value_2) (`.WorldLocation_5_A610825A49763CE01582F8BE4E12333F` (break `/Game/Blueprint/Struct_Tile` _value_2)) (`.Coordinates_8_53032BC04019C34375C23FA909D32976` (break `/Game/Blueprint/Struct_Tile` _value_2)) (`.TileActor_27_C837385A4995B3A36BD7829C414865E1` (break `/Game/Blueprint/Struct_Tile` _value_2)) (`.Cost_25_2C52E69A47A40DBB903D63AE9718D093` (break `/Game/Blueprint/Struct_Tile` _value_2)) 0 _estimatedcost_2 _estimatedcost_2)))
      (:`then_1`
        (bind _output_get (set `local.CurrentTile` (`local.Start`)))
        (`KismetArrayLibrary.Array_AddUnique` _openset _output_get)
        (while (> (`KismetArrayLibrary.Array_Length` _openset) 0)
          (set `local.OpenSetCheapest` (`|GetArrayItem` (`local.OpenSet`)))
          (for _array_element_2 (`local.OpenSet`)
            (bind _value_5 (`BlueprintMapLibrary.Map_Find` _tilesdata _array_element_2))
            (if (< (`.FinalCost_21_A36BEAB94CFF52A106DACA90997CC7A2` (break `/Game/Blueprint/Struct_Tile` _value_5)) (`.FinalCost_21_A36BEAB94CFF52A106DACA90997CC7A2` (break `/Game/Blueprint/Struct_Tile` _value)))
              (set `local.OpenSetCheapest` _array_element_2 :!label _label)
              (elif (== (`.FinalCost_21_A36BEAB94CFF52A106DACA90997CC7A2` (break `/Game/Blueprint/Struct_Tile` _value_5)) (`.FinalCost_21_A36BEAB94CFF52A106DACA90997CC7A2` (break `/Game/Blueprint/Struct_Tile` _value)))
                (if (< (`.EstimatedCostToGoal_19_02423FE3400E4EB9969D35B9CA7A6A79` (break `/Game/Blueprint/Struct_Tile` _value_5)) (`.EstimatedCostToGoal_19_02423FE3400E4EB9969D35B9CA7A6A79` (break `/Game/Blueprint/Struct_Tile` _value)))
                  (goto _label)))))
          (`|ExecutionSequence`
            (:`then_0`
              (bind _output_get_2 (set `local.CurrentTile` (`local.OpenSetCheapest`)))
              (`KismetArrayLibrary.Array_RemoveItem` (`local.OpenSet`) _output_get_2)
              (`KismetArrayLibrary.Array_AddUnique` (`local.ClosedSet`) _output_get_2))
            (:`then_1`
              (for _array_element_3 (`self.GetTileNeighbours` (`local.CurrentTile`))
                (bind _output_get_3 (set `local.CurrentNeighbour` _array_element_3))
                (if (not (`KismetArrayLibrary.Array_Contains` (`local.ClosedSet`) _output_get_3))
                  (set `local.CurrentNeighbourCostFromStart` (+ (`.CostFromStart_17_1A89801540D7C595984E6BAD394633A3` (break `/Game/Blueprint/Struct_Tile` (`BlueprintMapLibrary.Map_Find` _tilesdata_3 (`local.CurrentTile`)))) (`.CostFromStart_17_1A89801540D7C595984E6BAD394633A3` (break `/Game/Blueprint/Struct_Tile` (`BlueprintMapLibrary.Map_Find` _tilesdata_3 (`local.CurrentNeighbour`))))))
                  (if (`KismetArrayLibrary.Array_Contains` (`local.OpenSet`) (`local.CurrentNeighbour`))
                    (if (< (`local.CurrentNeighbourCostFromStart`) (`.CostFromStart_17_1A89801540D7C595984E6BAD394633A3` (break `/Game/Blueprint/Struct_Tile` _value_3)))
                      (`BlueprintMapLibrary.Map_Add` (`self.TilesData`) (`local.CurrentNeighbour`) (make `/Game/Blueprint/Struct_Tile` (break `/Game/Blueprint/Struct_Tile` _value_3) (`.WorldLocation_5_A610825A49763CE01582F8BE4E12333F` (break `/Game/Blueprint/Struct_Tile` _value_3)) (`.Coordinates_8_53032BC04019C34375C23FA909D32976` (break `/Game/Blueprint/Struct_Tile` _value_3)) (`.TileActor_27_C837385A4995B3A36BD7829C414865E1` (break `/Game/Blueprint/Struct_Tile` _value_3)) (`.Cost_25_2C52E69A47A40DBB903D63AE9718D093` (break `/Game/Blueprint/Struct_Tile` _value_3)) (`local.CurrentNeighbourCostFromStart`) _estimatedcost (+ _estimatedcost _estimatedcost) (`local.CurrentTile`)) :!label _label_2)
                      (if (== (`local.CurrentNeighbour`) (`local.Goal`) :`ErrorTolerance` 0.0001)
                        (set `self.Path` (`self.RetracePath` (`local.Goal`) (`local.Start`)))
                        (return)))
                    (else
                      (`KismetArrayLibrary.Array_AddUnique` (`local.OpenSet`) (`local.CurrentNeighbour`))
                      (goto _label_2))))))))))))

(fn `GenerateMapDataFromWorld`
  (locals (X :type Integer) (Y :type Integer))
  (bind _tilesize (`self.TileSize`))
  (bind _returnvalue (`KismetMathLibrary.MakeVector2D` (`KismetMathLibrary.Conv_IntToDouble` (`local.X`)) (`KismetMathLibrary.Conv_IntToDouble` (`local.Y`))))
  (bind _returnvalue_2 (`KismetMathLibrary.MakeVector2D` (`KismetMathLibrary.Conv_IntToDouble` (`local.X`)) (`KismetMathLibrary.Conv_IntToDouble` (`local.Y`))))
  (bind _returnvalue_3 (`KismetMathLibrary.MakeVector2D` (`KismetMathLibrary.Conv_IntToDouble` (`local.X`)) (`KismetMathLibrary.Conv_IntToDouble` (`local.Y`))))
  (bind (_horizontal _vertical) (`self.GetTileNumber`))
  (for _index (range _horizontal)
    (set `local.X` _index)
    (for _index_2 (range _vertical)
      (set `local.Y` _index_2)
      (bind _bottomleft (`self.GetBottomLeft`))
      ;[1 1 1] Ground
      (bind _output_get (set `self.TileLocation` (+ _bottomleft (+ (* (`SceneComponent.GetRightVector` (`self.Scene`)) (* (`local.X`) (* 2 (`self.TileSize`)))) (`KismetMathLibrary.MakeVector` _tilesize)) (+ (`KismetMathLibrary.MakeVector` 0.0 _tilesize) (* (`SceneComponent.GetForwardVector` (`self.Scene`)) (* (`local.Y`) (* 2 (`self.TileSize`))))))))
      (bind _iscollision (`self.TileSphereTrace` _output_get "TraceTypeQuery3"))
      (if _iscollision
        ;[1 0.3351 0 0.33] Obstacles
        (bind (_iscollision_2 _collidedactor) (`self.TileSphereTrace` (`self.TileLocation`) "TraceTypeQuery4"))
        (if (not _iscollision_2)
          (bind _cost (`self.GetTileCost` "NewEnumerator1"))
          (`BlueprintMapLibrary.Map_Add` (`self.TilesData`) _returnvalue (make `/Game/Blueprint/Struct_Tile` "NewEnumerator1" (`self.TileLocation`) _returnvalue null _cost))
          (else
            (bind _asbp_obstacle (cast `/Game/Blueprint/BP_Obstacle` _collidedactor))
            (bind _groundtype (`/Game/Blueprint/BP_Obstacle.GroundType` _asbp_obstacle))
            (bind _cost_2 (`self.GetTileCost` _groundtype))
            (`BlueprintMapLibrary.Map_Add` (`self.TilesData`) _returnvalue_3 (make `/Game/Blueprint/Struct_Tile` _groundtype (`self.TileLocation`) _returnvalue_3 null _cost_2))))
        (else
          (bind _cost_3 (`self.GetTileCost` "NewEnumerator0"))
          (`BlueprintMapLibrary.Map_Add` (`self.TilesData`) _returnvalue_2 (make `/Game/Blueprint/Struct_Tile` "NewEnumerator0" (`self.TileLocation`) _returnvalue_2 null _cost_3)))))))

(fn `GetBottomLeft`
  (returns (BottomLeft :type "Vector Structure"))
  (bind _scene (`self.Scene`))
  (bind (_gridsizeworld_x _gridsizeworld_y) (`KismetMathLibrary.BreakVector2D` (`self.GridSizeWorld`)))
  (return (- (- (`SceneComponent.K2_GetComponentLocation` _scene) (* (`SceneComponent.GetForwardVector` _scene) _gridsizeworld_x)) (* _gridsizeworld_y (`SceneComponent.GetRightVector` _scene)))))

(fn `GetEstimatedCostToGoal`
  (params (CurrentCoords :type "Vector2D Structure") (GoalCoords :type "Vector2D Structure"))
  (returns (EstimatedCost :type Integer))
  (bind (_returnvalue_x _returnvalue_y) (`KismetMathLibrary.BreakVector2D` (- CurrentCoords GoalCoords)))
  (return (`KismetMathLibrary.Round` (+ (`KismetMathLibrary.Abs` _returnvalue_x) (`KismetMathLibrary.Abs` _returnvalue_y)))))

(fn `GetTileCost`
  (params (Ground :type "/Game/Blueprint/Enum_GroundType Enum" :default "NewEnumerator0"))
  (returns (Cost :type Integer))
  (switch `/Game/Blueprint/Enum_GroundType` Ground
    (:`NewEnumerator0`
      (return 0))
    (:`NewEnumerator1`
      (return 25))
    (:`NewEnumerator2`
      (return 50))))

(fn `GetTileNeighbours`
  (params (Coordinates :type "Vector2D Structure"))
  (returns (Neighbours :type "Array of Vector2D Structure"))
  (locals (PossibleNeighbours :type "Array of Vector2D Structure") (OutNeighbours :type "Array of Vector2D Structure"))
  (bind _output_get (set `local.PossibleNeighbours` (`|MakeArray` (1.0 0.0) (0.0 1.0) (-1.0 0.0) (0.0 -1.0) :!type "Vector2D Structure")))
  (for _array_element _output_get
    (bind (_value _returnvalue) (`BlueprintMapLibrary.Map_Find` (`self.TilesData`) (+ _array_element Coordinates)))
    (if _returnvalue
      (if (and (`|EnumInequality` (break `/Game/Blueprint/Struct_Tile` _value) "NewEnumerator2") (`|EnumInequality` (break `/Game/Blueprint/Struct_Tile` _value) "NewEnumerator0"))
        (`KismetArrayLibrary.Array_AddUnique` (`local.OutNeighbours`) (`.Coordinates_8_53032BC04019C34375C23FA909D32976` (break `/Game/Blueprint/Struct_Tile` _value))))))
  (return (`local.OutNeighbours`)))

(fn `GetTileNumber`
  (returns (Horizontal :type Integer) (Vertical :type Integer))
  (bind (_gridsizeworld_x _gridsizeworld_y) (`KismetMathLibrary.BreakVector2D` (`self.GridSizeWorld`)))
  (bind _tilesize (`self.TileSize`))
  (return (`KismetMathLibrary.FTrunc` (/ _gridsizeworld_x _tilesize)) (`KismetMathLibrary.FTrunc` (/ _gridsizeworld_y _tilesize))))

(fn `HighlightCurrentPath`
  (params (IsForHighlight :type Boolean))
  (for _array_element (`self.Path`)
    (bind _value (`BlueprintMapLibrary.Map_Find` (`self.TilesData`) _array_element))
    (`/Engine/EditorBlueprintResources/StandardMacros.IsValid` (`.TileActor_27_C837385A4995B3A36BD7829C414865E1` (break `/Game/Blueprint/Struct_Tile` _value))
      (:`Is Valid`
        (`/Game/Blueprint/BP_Tile.OnPutInPath` (`.TileActor_27_C837385A4995B3A36BD7829C414865E1` (break `/Game/Blueprint/Struct_Tile` _value)) IsForHighlight)))))

(fn `RetracePath`
  (params (ReversedStart :type "Vector2D Structure") (ReversedGoal :type "Vector2D Structure"))
  (returns (Path :type "Array of Vector2D Structure"))
  (locals (CurrentTile :type "Vector2D Structure") (ReversedPath :type "Array of Vector2D Structure") (OutPath :type "Array of Vector2D Structure"))
  (bind _output_get (set `local.CurrentTile` ReversedStart))
  (while (!= _output_get ReversedGoal :`ErrorTolerance` 0.0001)
    (`KismetArrayLibrary.Array_AddUnique` (`local.ReversedPath`) (`local.CurrentTile`))
    (set `local.CurrentTile` (`.PreviousTile_26_0828B184438F758BF286FF943E233B76` (break `/Game/Blueprint/Struct_Tile` (`BlueprintMapLibrary.Map_Find` (`self.TilesData`) (`local.CurrentTile`))))))
  (bind (_arrayindex _arrayelement) (`/Engine/EditorBlueprintResources/StandardMacros.ReverseForEachLoop` (`local.ReversedPath`))
    (:`LoopBody`
      (`KismetArrayLibrary.Array_AddUnique` (`local.OutPath`) _arrayelement))
    (:`Completed`
      (return (`local.OutPath`)))))

(fn `TileSphereTrace`
  (params (Location :type "Vector Structure") (TraceChannel :type "ETraceTypeQuery Enum" :default "TraceTypeQuery1"))
  (returns (IsCollision :type Boolean) (CollidedActor :type "Actor Object Reference"))
  (locals (Collision :type Boolean) (HitActor :type "Actor Object Reference"))
  (bind (_outhit _returnvalue) (`KismetSystemLibrary.SphereTraceSingle` Location (+ Location (0.01 0.0 0.0)) 50.0 TraceChannel))
  (return _returnvalue (`.HitActor` (`GameplayStatics.BreakHitResult` _outhit))))

(fn `UserConstructionScript`
  (bind (_gridsizeworld_x _gridsizeworld_y) (`KismetMathLibrary.BreakVector2D` (`self.GridSizeWorld`)))
  (`KismetSystemLibrary.FlushPersistentDebugLines`)
  (bind _output_get (set `self.GridLocation` (`SceneComponent.K2_GetComponentLocation` (`self.Scene`))))
  (`KismetSystemLibrary.DrawDebugBox` _output_get (`KismetMathLibrary.MakeVector` _gridsizeworld_y _gridsizeworld_x) (`self.GridColor`) (struct) 100000.0 10.0)
  (`self.GenerateMapDataFromWorld`)
  (`self.DrawTiles`))