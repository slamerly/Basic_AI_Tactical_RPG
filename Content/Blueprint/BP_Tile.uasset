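; Clickable tile actor for a grid, showing its ground type, hover and selection state.
; It looks up its data in the Grid's TilesData by coordinates, then sets material parameters for color, hover brightening and selection highlight.
; After a short BeginPlay delay it colors and scales itself from the grid's tile size.
; Hover and click notify the Grid; clicking only selects, as the FlipFlop toggle is unconnected.
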(event `self.ReceiveBeginPlay`
  (`KismetSystemLibrary.Delay` 0.5)
  (`self.SetTileColor`)
  (`self.SetTileSize`))

(event `self.StaticMesh.OnBeginCursorOver`
  (params (TouchedComponent :type "PrimitiveComponent Object Reference"))
  (set `self.IsHover` true)
  (`self.SetTileColor`)
  (`/Game/Blueprint/BP_Grid.OnCurrentlyHoveredTile` (`self.Grid`) self))

(event `self.StaticMesh.OnEndCursorOver`
  (params (TouchedComponent :type "PrimitiveComponent Object Reference"))
  (set `self.IsHover` false)
  (`self.SetTileColor`))

(event `OnSelectTile`
  (set `self.IsSelected` true)
  (`self.SetTileColor`)
  (`/Game/Blueprint/BP_Grid.OnNewTileSelected` (`self.Grid`) self))

(event `OnUnselectTile`
  (set `self.IsSelected` false)
  (`self.SetTileColor`))

(event `self.StaticMesh.OnClicked`
  (params (TouchedComponent :type "PrimitiveComponent Object Reference") (ButtonPressed :type "Key Structure"))
  (`self.OnSelectTile`))

(fn `GetTileData`
  (returns (ValueGroundType :type "/Game/Blueprint/Enum_GroundType Enum") (ValueWorldLocation :type "Vector Structure") (ValueCoordinates :type "Vector2D Structure"))
  (bind _value (`BlueprintMapLibrary.Map_Find` (`/Game/Blueprint/BP_Grid.TilesData` (`self.Grid`)) (`self.GridCoordinates`)))
  (return (break `/Game/Blueprint/Struct_Tile` _value) (`.WorldLocation_5_A610825A49763CE01582F8BE4E12333F` (break `/Game/Blueprint/Struct_Tile` _value)) (`.Coordinates_8_53032BC04019C34375C23FA909D32976` (break `/Game/Blueprint/Struct_Tile` _value))))

(fn `SetTileColor`
  (bind _staticmesh (`self.StaticMesh`))
  (bind _valuegroundtype (`self.GetTileData`))
  (switch `/Game/Blueprint/Enum_GroundType` _valuegroundtype
    (:`NewEnumerator0`
      (set `self.TileColor` (struct :`R` 1.0 :`G` 1.0 :`B` 1.0 :`A` 1.0)))
    (:`NewEnumerator1`
      (set `self.TileColor` (struct :`R` 0.078125 :`G` 0.03177 :`A` 1.0)))
    (:`NewEnumerator2`
      (set `self.TileColor` (struct))))
  (if (`self.IsHover`)
    (set `self.TileColor` (* (`self.TileColor`) 5.0)))
  (`MeshComponent.SetVectorParameterValueOnMaterials` (`self.StaticMesh`) "TileColor" (`KismetMathLibrary.Conv_LinearColorToVector` (`self.TileColor`)))
  (if (`self.IsSelected`)
    (`MeshComponent.SetScalarParameterValueOnMaterials` _staticmesh "SelectionAlpha" 1.0)
    (else
      (`MeshComponent.SetScalarParameterValueOnMaterials` _staticmesh "SelectionAlpha" 0.0))))

(fn `SetTileSize`
  (bind _staticmesh (`self.StaticMesh`))
  (bind (_returnvalue_x _returnvalue_y) (`KismetMathLibrary.BreakVector` (* (`SceneComponent.K2_GetComponentScale` _staticmesh) (/ (`/Game/Blueprint/BP_Grid.TileSize` (`self.Grid`)) 50.0))))
  (`SceneComponent.SetWorldScale3D` _staticmesh (`KismetMathLibrary.MakeVector` _returnvalue_x _returnvalue_y)))

(fn `UserConstructionScript`)