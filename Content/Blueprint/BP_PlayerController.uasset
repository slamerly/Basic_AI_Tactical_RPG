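; BP_PlayerController is a player controller that tracks the selected unit and relays movement paths to it.
; It enables mouse-over and click events on BeginPlay.
; NewUnitSelected notifies the previous unit that it is unselected, then stores the new one.
; OnNewPathAvailable stores the incoming path and tells the selected unit, if valid, to move along it.
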(event `self.ReceiveBeginPlay`
  (set `self.bEnableMouseOverEvents` true)
  (set `self.bEnableClickEvents` true))

(event `NewUnitSelected`
  (params (NewSelectedUnit :type "/Game/Blueprint/BP_Unit Object Reference"))
  (bind _selectedunit (`self.SelectedUnit`))
  (`/Engine/EditorBlueprintResources/StandardMacros.IsValid` _selectedunit
    (:`Is Valid`
      (`/Game/Blueprint/BP_Unit.OnUnitUnselected` _selectedunit))
    (:`Is Not Valid`
      _))
  (set `self.SelectedUnit` NewSelectedUnit))

(event `OnNewPathAvailable`
  (params (NewPath :type "Array of Vector2D Structure"))
  (bind _selectedunit (`self.SelectedUnit`))
  (bind _output_get (set `self.Path` NewPath))
  (`/Engine/EditorBlueprintResources/StandardMacros.IsValid` _selectedunit
    (:`Is Valid`
      (`/Game/Blueprint/BP_Unit.OnMoveAlongPath` _selectedunit _output_get))))

(fn `UserConstructionScript`)