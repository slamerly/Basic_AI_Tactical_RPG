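; BP_Unit is a clickable grid unit that can be selected and moved along a tile path.
; On BeginPlay it finds BP_Grid, snaps to the nearest tile in TilesData and stores those coordinates.
; Clicking either cube toggles selection through BP_PlayerController, with debug prints on select and unselect.
; Movement rebuilds the grid's shared spline from path tiles, raised by capsule half-height, then a timeline drives position and rotation along it.
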(event `self.ReceiveBeginPlay`
  (bind _outactors (`GameplayStatics.GetAllActorsOfClass` "/Game/Blueprint/BP_Grid.BP_Grid_C"))
  (set `self.Grid` (`|GetArrayItem` _outactors))
  (`self.SetCoordsAndSnap`)
  (bind _asbp_player_controller (cast `/Game/Blueprint/BP_PlayerController` (`GameplayStatics.GetPlayerController` 0)))
  (set `self.PlayerController` _asbp_player_controller))

(event `OnUnitSelected`
  (`KismetSystemLibrary.PrintString` "Hello")
  (`KismetSystemLibrary.PrintString` (`KismetStringLibrary.Conv_VectorToString` (`SceneComponent.K2_GetComponentLocation` (`self.CapsuleComponent`))) true true (struct :`G` 0.66 :`B` 1.0 :`A` 1.0) 10.0))

(event `OnUnitUnselected`
  (`KismetSystemLibrary.PrintString` "Bye"))

(event `self.Cube.OnClicked`
  (params (TouchedComponent :type "PrimitiveComponent Object Reference") (ButtonPressed :type "Key Structure"))
  (if (!= (`/Game/Blueprint/BP_PlayerController.SelectedUnit` (`self.PlayerController`)) self) :!label _label
    (`/Game/Blueprint/BP_PlayerController.NewUnitSelected` (`self.PlayerController`) self)
    (`self.OnUnitSelected`)
    (else
      (`/Game/Blueprint/BP_PlayerController.NewUnitSelected` (`self.PlayerController`) null))))

(event `self.Cube1.OnClicked`
  (params (TouchedComponent :type "PrimitiveComponent Object Reference") (ButtonPressed :type "Key Structure"))
  (goto _label))

(event `OnMoveAlongPath`
  (params (Path :type "Array of Vector2D Structure"))
  (bind _spline (`/Game/Blueprint/BP_Grid.Spline` (`self.Grid`)))
  (bind _output_get (set `self.Path` Path))
  (set `self.Coordinates` (`|GetArrayItem` _output_get (`KismetArrayLibrary.Array_LastIndex` _output_get)))
  (`SplineComponent.ClearSplinePoints` (`/Game/Blueprint/BP_Grid.Spline` (`self.Grid`)) true)
  (for _array_element (`self.Path`)
    (bind _value (`BlueprintMapLibrary.Map_Find` (`/Game/Blueprint/BP_Grid.TilesData` (`self.Grid`)) _array_element))
    (`SplineComponent.AddSplinePoint` (`/Game/Blueprint/BP_Grid.Spline` (`self.Grid`)) (`KismetMathLibrary.MakeVector` (.x (`.WorldLocation_5_A610825A49763CE01582F8BE4E12333F` (break `/Game/Blueprint/Struct_Tile` _value))) (.y (`.WorldLocation_5_A610825A49763CE01582F8BE4E12333F` (break `/Game/Blueprint/Struct_Tile` _value))) (+ (.z (`.WorldLocation_5_A610825A49763CE01582F8BE4E12333F` (break `/Game/Blueprint/Struct_Tile` _value))) (`CapsuleComponent.CapsuleHalfHeight` (`self.CapsuleComponent`)))) "Local" true))
  (bind (_direction _movement) (`Timeline|PathTimeline` :!via `PlayFromStart`)
    (:`Update`
      (bind _returnvalue (* _movement (`SplineComponent.GetSplineLength` _spline)))
      (`self.K2_SetActorTransform` self (`KismetMathLibrary.MakeTransform` (`SplineComponent.GetLocationAtDistanceAlongSpline` _spline _returnvalue "World") (`SplineComponent.GetRotationAtDistanceAlongSpline` _spline _returnvalue "World")) false false))))

(fn `SetCoordsAndSnap`
  (locals (ClosestTileDistance :type "Float (double-precision)") (ClosestCoords :type "Vector2D Structure"))
  (bind _tilesdata (`/Game/Blueprint/BP_Grid.TilesData` (`self.Grid`)))
  (set `local.ClosestTileDistance` 999999.0)
  (bind _keys (`BlueprintMapLibrary.Map_Keys` _tilesdata))
  (for _array_element _keys
    (bind _returnvalue (`KismetMathLibrary.VSize` (- (`.WorldLocation_5_A610825A49763CE01582F8BE4E12333F` (break `/Game/Blueprint/Struct_Tile` (`BlueprintMapLibrary.Map_Find` _tilesdata _array_element))) (`self.K2_GetActorLocation` self))))
    (if (< _returnvalue (`local.ClosestTileDistance`))
      (set `local.ClosestTileDistance` _returnvalue)
      (set `local.ClosestCoords` _array_element)))
  (set `self.Coordinates` (`local.ClosestCoords`))
  (`self.K2_SetActorLocation` (`.WorldLocation_5_A610825A49763CE01582F8BE4E12333F` (break `/Game/Blueprint/Struct_Tile` (`BlueprintMapLibrary.Map_Find` (`/Game/Blueprint/BP_Grid.TilesData` (`self.Grid`)) (`local.ClosestCoords`))))))

(fn `UserConstructionScript`)